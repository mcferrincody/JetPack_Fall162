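; BP_Ring is a collectible ring that jumps to random spots in the play area at a fixed height.
; InitRing teleports it and re-arms its own timer, with the delay shrinking as the FP_GameMode level rises.
; When the player overlaps it before game over, it reports the pickup to the game mode and replaces itself with a new ring, which relocates on BeginPlay.
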(event `self.ReceiveBeginPlay`
  (bind _asfp_game_mode (cast `/Game/FirstPersonBP/Blueprints/BaseFPS/FP_GameMode` (`GameplayStatics.GetGameMode`)))
  (set `self.My_FP_GameMode` _asfp_game_mode)
  (`self.InitRing`))

(event `self.ReceiveActorBeginOverlap`
  (params (OtherActor :type "Actor Object Reference"))
  (if (and (== OtherActor (`GameplayStatics.GetPlayerCharacter` 0)) (not (`/Game/FirstPersonBP/Blueprints/BaseFPS/FP_GameMode.GameOver` (`self.My_FP_GameMode`))))
    (`/Game/FirstPersonBP/Blueprints/BaseFPS/FP_GameMode.Rings Collected` (`self.My_FP_GameMode`))
    (`self.K2_DestroyActor`)
    (`|SpawnActorFromClass` "BP_Ring_C" (`self.GetTransform`) "Undefined" "OverrideRootScale" null null)))

(fn `InitRing`
  (`self.K2_TeleportTo` (`KismetMathLibrary.MakeVector` (`KismetMathLibrary.RandomFloatInRange` -1800.0 1000.0) (`KismetMathLibrary.RandomFloatInRange` -1400.0 1400.0) 130.0))
  (`KismetSystemLibrary.K2_SetTimer` null "InitRing" (`KismetMathLibrary.Conv_IntToDouble` (- 6 (`/Game/FirstPersonBP/Blueprints/BaseFPS/FP_GameMode.Level` (`self.My_FP_GameMode`))))))

(fn `UserConstructionScript`)